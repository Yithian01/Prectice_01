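; BP_P38 is a player-controlled P38 aircraft pawn that rotates on input and fires rockets.
; Roll and Pitch axes apply clamped, frame-time-scaled local rotation to the static mesh, both using PitchSpeed.
; Pressing Fire spawns a BP_Rocket at the Arrow component's transform.
; Tick is empty and the forward AddMovementInput node is never run, so this graph does not move the plane.
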(event `InputAxis|Roll`
  (params (AxisValue :type "Float (single-precision)"))
  ; Roll & Pitch
  (`SceneComponent.K2_AddLocalRotation` (`self.StaticMesh`) (`KismetMathLibrary.MakeRotator` (* (`KismetMathLibrary.FClamp` AxisValue -1.0) (`GameplayStatics.GetWorldDeltaSeconds`) (`self.PitchSpeed`))) false false))

(event `InputAxis|Pitch`
  (params (AxisValue :type "Float (single-precision)"))
  ; Roll & Pitch
  (`SceneComponent.K2_AddLocalRotation` (`self.StaticMesh`) (`KismetMathLibrary.MakeRotator` 0.0 (* (`KismetMathLibrary.FClamp` AxisValue -1.0) (`GameplayStatics.GetWorldDeltaSeconds`) (`self.PitchSpeed`))) false false))

(event `self.ReceiveTick`
  (params (DeltaSeconds :type "Float (single-precision)"))
  ; Move
)

(event `InputAction|Fire`
  (params (Key :type "Key Structure"))
  (:`Pressed`
    (`|SpawnActorFromClass` "/Game/BP/BP_Rocket.BP_Rocket_C" (`SceneComponent.K2_GetComponentToWorld` (`self.Arrow`)) "Undefined" "MultiplyWithRoot" null null)))

(fn `UserConstructionScript`)